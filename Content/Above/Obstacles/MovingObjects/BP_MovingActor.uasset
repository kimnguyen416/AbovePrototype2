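; BP_MovingActor is a moving obstacle that damages the player character on contact.
; On BeginPlay it caches its location, then a timeline lerps the static mesh toward that start plus EndLocation, so EndLocation acts as a relative offset.
; The mesh moves without sweeping.
; A box overlap casts to BP_MC and subtracts a fixed amount directly from CurrentHealth.
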(event `self.ReceiveBeginPlay`
  (set `self.startLocation` (`self.K2_GetActorLocation`))
  (bind (_direction _newtrack_0) (`Timeline|Moving_Timeline`)
    (:`Update`
      (`SceneComponent.K2_SetWorldLocation` (`self.StaticMesh`) (`KismetMathLibrary.VLerp` (`self.startLocation`) (+ (`self.startLocation`) (`self.endLocation`)) _newtrack_0) false false))))

(event `self.Box.OnComponentBeginOverlap`
  (params (OverlappedComponent :type "PrimitiveComponent Object Reference") (OtherActor :type "Actor Object Reference") (OtherComp :type "PrimitiveComponent Object Reference") (OtherBodyIndex :type Integer) (bFromSweep :type Boolean) (SweepResult :type "HitResult Structure (by ref)"))
  (bind _asbp_mc (cast `/Game/Above/MainCharacter/BP_MC` OtherActor))
  (set `/Game/Above/MainCharacter/BP_MC.currentHealth` (- (`/Game/Above/MainCharacter/BP_MC.currentHealth` _asbp_mc) 10.0) _asbp_mc))

(fn `UserConstructionScript`)