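; Teleporting enemy that, on seeing the player through PawnSensing, darts between three patrol points and fires projectiles.
; BeginPlay caches the world locations of three position components and picks one at random.
; Patrol_Timeline updates lerp the actor toward that point, yaw it at the player and spawn BP_Projectile while ammo remains.
; A two-second Delay within the update picks another random point and refills the short burst.
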(event `self.PawnSensing.OnSeePawn`
  (params (Pawn :type "Pawn Object Reference"))
  (bind _maxbullet (`self.maxBullet`))
  (cast `/Game/Above/MainCharacter/BP_MC` Pawn)
  (`Timeline|Patrol_Timeline`
    (:`Update`
      (`|ExecutionSequence`
        (:`then_0`
          (`self.K2_SetActorLocation` (`KismetMathLibrary.VLerp` (`self.K2_GetActorLocation`) (`|GetArrayItem` (`self.PatrolPoints`) (`self.CurrentPatrol`)) 0.2))
          (if (`self.shoot?`)
            (`|SpawnActorFromClass` "/Game/Above/Obstacles/ShootingMachine/BP_Projectile.BP_Projectile_C" (`SceneComponent.K2_GetComponentToWorld` (`self.ShootHere`)) "Undefined" "OverrideRootScale" null null)
            (set `self.maxBullet` (- _maxbullet 1))
            (if (<= _maxbullet 0)
              (set `self.shoot?` false))))
        (:`then_1`
          (bind _asbp_mc (cast `/Game/Above/MainCharacter/BP_MC` (`GameplayStatics.GetPlayerCharacter` 0)))
          (`|ExecutionSequence`
            (:`then_0`
              (`self.K2_SetActorRotation` (`KismetMathLibrary.MakeRotator` 0.0 0.0 (.yaw (`KismetMathLibrary.FindLookAtRotation` (`self.K2_GetActorLocation`) (`self.K2_GetActorLocation` _asbp_mc)))))
              (`KismetSystemLibrary.Delay` 2.0)
              (`self.GetRandomLocation`)
              (set `self.maxBullet` 2)
              (set `self.shoot?` true))))))))

(event `self.ReceiveBeginPlay`
  ;[1 1 1] Player can teleport to 3 points
  (set `self.PatrolPoints` (`|MakeArray` (`SceneComponent.K2_GetComponentLocation` (`self.Position1`)) (`SceneComponent.K2_GetComponentLocation` (`self.Position2`)) (`SceneComponent.K2_GetComponentLocation` (`self.Position3`))))
  (`self.GetRandomLocation`))

(fn `GetRandomLocation`
  (set `self.CurrentPatrol` (`KismetMathLibrary.RandomInteger` (`KismetArrayLibrary.Array_Length` (`self.PatrolPoints`)))))

(fn `UserConstructionScript`)